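; PC_UMG is a player controller Blueprint that toggles a pause menu on the Pause input action.
; The stored widget reference acts as the toggle state: if empty, it creates and shows a menu widget, enables Game and UI input with the cursor, and pauses the game.
; If valid, it removes the widget and reverses those settings.
; Either way, it tells Character_FirstHourUMG to hide or restore its HUD.
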(event Input|ActionEvents|InputActionPause
  (params (Key :type Key%20Structure :default "None"))
  (bind _returnvalue (Game|GetPlayerController 0))
  ;[1 1 1] Pause menu
  (:Pressed
    (Utilities|IsValid (Variables|Default|GetPauseUIRef)
      (:Is%20Valid
        (Widget|RemovefromParent (Variables|Default|GetPauseUIRef))
        (Variables|Default|SetPauseUIRef 0)
        (Input|SetInputModeGameOnly (Game|GetPlayerController 0))
        (Variables|Default|SetbShowMouseCursor false)
        (Game|SetGamePaused false)
        (bind _ascharacter_first_hour_umg (Utilities|Casting|CastToCharacter_FirstHourUMG (Game|GetPlayerCharacter 0)))
        (Default|ToggleHUDon _ascharacter_first_hour_umg))
      (:Is%20Not%20Valid
        (bind _returnvalue_2 (UserInterface|CreateWidget "/Game/FirstHourUMG/Widgets/UMG_MainMenu.UMG_MainMenu_C"))
        (bind _output_get (Variables|Default|SetPauseUIRef _returnvalue_2))
        (UserInterface|Viewport|AddtoViewport _output_get 0)
        (Input|SetInputModeGameandUI _returnvalue 0 "DoNotLock" true)
        (Variables|/Script/Engine.PlayerController|SetbShowMouseCursor _returnvalue true)
        (Game|SetGamePaused true)
        (bind _ascharacter_first_hour_umg_2 (Utilities|Casting|CastToCharacter_FirstHourUMG (Game|GetPlayerCharacter 0)))
        (Default|ToggleHUDOff _ascharacter_first_hour_umg_2)))))

(fn ConstructionScript)